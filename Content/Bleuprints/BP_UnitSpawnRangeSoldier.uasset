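; Ranged soldier unit for what appears to be an RTS, with its own health and damage and gathering disabled.
; Sphere overlaps track enemy soldiers in an array; a looping timer turns the unit toward the nearest, applies direct damage without projectiles and destroys it on low health.
; Tick drives AI MoveToLocation toward the destination, with a wider stop radius for warehouses, and shows a cylinder while selected.
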(event `self.ReceiveBeginPlay`
  ;[1 1 1] make soldier unable to gather
  (set `self.GatheringSpeed` 0.0)
  (set `self.Health` 225.0)
  (set `self.AttackDmg` 15.0)
  (`KismetSystemLibrary.K2_SetTimerDelegate` (delegate `Attack closest units`) 1.5 true))

(event `Attack closest units`
  (bind _unitenemyarray (`self.UnitEnemyArray`))
  (bind (_distance _returnvalue) (`GameplayStatics.FindNearestActor` (`self.K2_GetActorLocation` self) _unitenemyarray))
  ;[1 1 1] Attack closest unit
  (if (> (`KismetArrayLibrary.Array_Length` _unitenemyarray) 0)
    (if (`KismetSystemLibrary.IsValid` _returnvalue)
      (bind _asbp_unit_spawn_enemy_soldier (cast `/Game/Bleuprints/BP_UnitSpawnEnemySoldier` _returnvalue))
      (set `self.DestinationOfTargetToLookAt` (`self.K2_GetActorLocation` _asbp_unit_spawn_enemy_soldier))
      (`self.TurnToLocation` 0.0)
      (bind _returnvalue_2 (- (`UnitSpawn.Health` _asbp_unit_spawn_enemy_soldier) (`self.AttackDmg`)))
      (set `UnitSpawn.Health` _returnvalue_2 _asbp_unit_spawn_enemy_soldier)
      (if (<= _returnvalue_2 0.0)
        (`self.K2_DestroyActor` _asbp_unit_spawn_enemy_soldier)))))

(event `self.ReceiveTick`
  (params (DeltaSeconds :type "Float (single-precision)"))
  (bind _returnvalue (not (`self.bSelected`)))
  (`self.MoveToDestination`)
  (if _returnvalue
    _
    (else
      _))
  (`SceneComponent.SetHiddenInGame` (`self.Cylinder`) _returnvalue false))

(event `self.Sphere.OnComponentBeginOverlap`
  (params (OverlappedComponent :type "PrimitiveComponent Object Reference") (OtherActor :type "Actor Object Reference") (OtherComp :type "PrimitiveComponent Object Reference") (OtherBodyIndex :type Integer) (bFromSweep :type Boolean) (SweepResult :type "HitResult Structure (by ref)"))
  ;[1 1 1] Add Units closed to me to arrays
  (if (== (`GameplayStatics.GetObjectClass` OtherActor) "/Game/Bleuprints/BP_UnitSpawnEnemySoldier.BP_UnitSpawnEnemySoldier_C")
    (bind _asbp_unit_spawn_enemy_soldier (cast `/Game/Bleuprints/BP_UnitSpawnEnemySoldier` OtherActor))
    (`KismetArrayLibrary.Array_Add` (`self.UnitEnemyArray`) _asbp_unit_spawn_enemy_soldier)))

(event `self.Sphere.OnComponentEndOverlap`
  (params (OverlappedComponent :type "PrimitiveComponent Object Reference") (OtherActor :type "Actor Object Reference") (OtherComp :type "PrimitiveComponent Object Reference") (OtherBodyIndex :type Integer))
  ;[1 1 1] Add Units closed to me to arrays
  (if (== (`GameplayStatics.GetObjectClass` OtherActor) "/Game/Bleuprints/BP_UnitSpawnEnemySoldier.BP_UnitSpawnEnemySoldier_C")
    (bind _asbp_unit_spawn_enemy_soldier (cast `/Game/Bleuprints/BP_UnitSpawnEnemySoldier` OtherActor))
    (`KismetArrayLibrary.Array_RemoveItem` (`self.UnitEnemyArray`) _asbp_unit_spawn_enemy_soldier)))

(fn `AcceptableRadiusOfMove`
  (if (`self.bIfWarehouse`)
    (set `self.RadiusStopMove` 650.0)
    (else
      (set `self.RadiusStopMove` 1.0)))
  (return))

(fn `MoveToDestination`
  (bind _destination (`self.Destination`))
  (bind _radiusstopmove (`self.RadiusStopMove`))
  (bind _returnvalue (`AIBlueprintHelperLibrary.GetAIController` self))
  (if (`self.bUnitMove`)
    (if (`self.bIfTree`)
      (set `self.bUnitMove` false :!label _label)
      (set `self.bIfTree` false)
      (set `self.bIfRock` false)
      (if (`self.FollowUnitToAttack`)
        (if (`KismetSystemLibrary.IsValid` _returnvalue) :!label _label_2
          (set `CharacterMovementComponent.MaxWalkSpeed` 300.0 (`self.CharacterMovement`))
          (`self.AcceptableRadiusOfMove`)
          (`AIController.MoveToLocation` _returnvalue _destination _radiusstopmove true true false true null true)
          (if (== _destination (`self.K2_GetActorLocation` self) :`ErrorTolerance` _radiusstopmove)
            (`SkeletalMeshComponent.SetAnimation` (`self.Mesh`) "/Game/Mannequin/Animations/ThirdPersonIdle.ThirdPersonIdle")
            (if (`self.bIfWarehouse`)
              (if (`KismetSystemLibrary.IsValid` (`self.ClickedTree`))
                (set `self.bUnitMove` true :!label _label_3)
                (elif (`KismetSystemLibrary.IsValid` (`self.ClickedRock`))
                  (goto _label_3)
                  (else
                    _)))
              (else
                (set `self.bUnitMove` false)))
            (return)
            (else
              (return)))
          (else
            _)))
      (elif (`self.bIfRock`)
        (goto _label)
        (elif (== _destination (`KismetMathLibrary.Vector_Zero`) :`ErrorTolerance` 1.0)
          _
          (else
            (goto _label_2)))))
    (else
      (goto _label)))
  (return))

(fn `TurnToLocation`
  (params (DeltaTime :type "Float (double-precision)"))
  (`self.K2_SetActorRotation` self (`KismetMathLibrary.FindLookAtRotation` (`self.K2_GetActorLocation` self) (`self.DestinationOfTargetToLookAt`)) false)
  (return))

(fn `UserConstructionScript`)