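; BP_UnitSpawn is a selectable unit that moves by AI MoveToLocation and automatically fights nearby enemy soldiers.
; Sphere overlaps maintain an enemy array; a looping timer damages the nearest, destroys it at depleted health, and sets its location as Destination.
; Tick drives MoveToDestination, which idles the unit on arrival or keeps it active for warehouse runs with a clicked tree or rock.
; Per-target stop radii are disconnected, leaving one small radius.
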(event `self.ReceiveBeginPlay`
  (`KismetSystemLibrary.K2_SetTimerDelegate` (delegate `Attack closest units`) 1.5 true)
  (set `self.UnitCylinder` (`self.Cylinder`))
  ;[1 1 1] bt need
  (set `self.UnitCharacterMovement` (`self.CharacterMovement`)))

(event `Attack closest units`
  (bind _unitenemyarray (`self.UnitEnemyArray`))
  (bind (_distance _returnvalue) (`GameplayStatics.FindNearestActor` (`self.K2_GetActorLocation` self) _unitenemyarray))
  ;[1 1 1] Attack closest unit
  (if (> (`KismetArrayLibrary.Array_Length` _unitenemyarray) 0)
    (set `self.RunAwayFromEnemy` true)
    (if (`KismetSystemLibrary.IsValid` _returnvalue)
      (bind _asbp_unit_spawn_enemy_soldier (cast `/Game/Bleuprints/BP_UnitSpawnEnemySoldier` _returnvalue))
      (set `self.Destination` (`self.K2_GetActorLocation` _asbp_unit_spawn_enemy_soldier))
      (bind _returnvalue_2 (- (`UnitSpawn.Health` _asbp_unit_spawn_enemy_soldier) (`self.AttackDmg`)))
      (set `UnitSpawn.Health` _returnvalue_2 _asbp_unit_spawn_enemy_soldier)
      (if (<= _returnvalue_2 0.0)
        (`self.K2_DestroyActor` _asbp_unit_spawn_enemy_soldier)))
    (else
      (set `self.RunAwayFromEnemy` false))))

(event `self.ReceiveTick`
  (params (DeltaSeconds :type "Float (single-precision)"))
  (`self.MoveToDestination`))

(event `self.Sphere.OnComponentBeginOverlap`
  (params (OverlappedComponent :type "PrimitiveComponent Object Reference") (OtherActor :type "Actor Object Reference") (OtherComp :type "PrimitiveComponent Object Reference") (OtherBodyIndex :type Integer) (bFromSweep :type Boolean) (SweepResult :type "HitResult Structure (by ref)"))
  ;[1 1 1] Add Units closed to me to arrays
  (if (== (`GameplayStatics.GetObjectClass` OtherActor) "/Game/Bleuprints/BP_UnitSpawnEnemySoldier.BP_UnitSpawnEnemySoldier_C")
    (bind _asbp_unit_spawn_enemy_soldier (cast `/Game/Bleuprints/BP_UnitSpawnEnemySoldier` OtherActor))
    (`KismetArrayLibrary.Array_Add` (`self.UnitEnemyArray`) _asbp_unit_spawn_enemy_soldier)))

(event `self.Sphere.OnComponentEndOverlap`
  (params (OverlappedComponent :type "PrimitiveComponent Object Reference") (OtherActor :type "Actor Object Reference") (OtherComp :type "PrimitiveComponent Object Reference") (OtherBodyIndex :type Integer))
  ;[1 1 1] Add Units closed to me to arrays
  (if (== (`GameplayStatics.GetObjectClass` OtherActor) "/Game/Bleuprints/BP_UnitSpawnEnemySoldier.BP_UnitSpawnEnemySoldier_C")
    (bind _asbp_unit_spawn_enemy_soldier (cast `/Game/Bleuprints/BP_UnitSpawnEnemySoldier` OtherActor))
    (`KismetArrayLibrary.Array_RemoveItem` (`self.UnitEnemyArray`) _asbp_unit_spawn_enemy_soldier)))

(fn `AcceptableRadiusOfMove`
  (if (`self.bIfTree`)
    _
    (elif (`self.bIfRock`)
      _
      (elif (`self.bIfWarehouse`)
        _
        (else
          _))))
  (set `self.RadiusStopMove` 1.0)
  (return))

(fn `MoveToDestination`
  (bind _destination (`self.Destination`))
  (bind _radiusstopmove (`self.RadiusStopMove`))
  (bind _returnvalue (`AIBlueprintHelperLibrary.GetAIController` self))
  (if (`self.bUnitMove`)
    (if (== _destination (`KismetMathLibrary.Vector_Zero`) :`ErrorTolerance` 1.0)
      (if (`self.RunAwayFromEnemy`) :!label _label
        (if (`KismetSystemLibrary.IsValid` _returnvalue) :!label _label_2
          (set `CharacterMovementComponent.MaxWalkSpeed` 300.0 (`self.CharacterMovement`))
          (`self.AcceptableRadiusOfMove`)
          (`AIController.MoveToLocation` _returnvalue _destination _radiusstopmove true true false true null true)
          (if (== _destination (`self.K2_GetActorLocation` self) :`ErrorTolerance` _radiusstopmove)
            (`SkeletalMeshComponent.SetAnimation` (`self.Mesh`) "/Game/Mannequin/Animations/ThirdPersonIdle.ThirdPersonIdle")
            (if (`self.bIfWarehouse`)
              (if (`KismetSystemLibrary.IsValid` (`self.ClickedTree`))
                (set `self.bUnitMove` true :!label _label_3)
                (elif (`KismetSystemLibrary.IsValid` (`self.ClickedRock`))
                  (goto _label_3)
                  (else
                    _)))
              (else
                (set `self.bUnitMove` false))))))
      (else
        (goto _label_2)))
    (else
      (goto _label)))
  (return))

(fn `UserConstructionScript`
  (`self.SpawnDefaultController` self)
  (set `self.AIControllerClass` "/Game/Bleuprints/UnitController.UnitController_C"))