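; Player camera controller pawn that holds input-driven state for a wheel axis and a building-connection mode.
; Holding Left Alt sets a wheel lock flag, while Alt+wheel actions step the wheel axis value up or down.
; A Shift+Alt action toggles ConnectBuildings and prints the new state.
; Unconnected leftover logic sketches a mouse-drag arrow from the click point to the deprojected cursor position, but never runs.
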(event `self.ReceiveBeginPlay`)

(event `self.ReceiveTick`
  (params (DeltaSeconds :type "Float (single-precision)")))

(event `Key|LeftAlt`
  (params (Key :type "Key Structure"))
  (:`Pressed`
    (set `self.bWheelLock` true))
  (:`Released`
    (set `self.bWheelLock` false)))

(event `InputAction|AltMouseWheelUp`
  (params (Key :type "Key Structure"))
  (:`Pressed`
    (set `self.WheelAxis` (+ (`self.WheelAxis`) 5.0))))

(event `InputAction|AltMouseWheelDown`
  (params (Key :type "Key Structure"))
  (:`Pressed`
    (set `self.WheelAxis` (+ (`self.WheelAxis`) -5.0))))

(event `InputAction|LeftShift+Alt`
  (params (Key :type "Key Structure"))
  (:`Pressed`
    (if (`self.bConnectBuildings`)
      (bind _output_get (set `self.bConnectBuildings` false))
      (`KismetSystemLibrary.PrintString` (`KismetStringLibrary.Conv_BoolToString` _output_get))
      (else
        (bind _output_get_2 (set `self.bConnectBuildings` true))
        (`KismetSystemLibrary.PrintString` (`KismetStringLibrary.Conv_BoolToString` _output_get_2))))))

(fn `UserConstructionScript`)