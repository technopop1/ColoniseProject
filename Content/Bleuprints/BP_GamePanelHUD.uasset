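; HUD Blueprint that creates the game panel and object HP widgets and handles drag-box unit selection.
; On BeginPlay it adds the widgets to the viewport, sharing the panel's bottom shop with the first of two HP widgets.
; While dragging, DrawHUD draws a translucent rectangle and gathers UnitSpawn actors inside it.
; StopSelection clears the player pawn's selection, adds those units and calls their CylinderHideShow.
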(event `self.ReceiveBeginPlay`
  (bind _returnvalue (`|CreateWidget` "/Game/Bleuprints/BP_GamePanelWidgetHUD.BP_GamePanelWidgetHUD_C"))
  (`UserWidget.AddToViewport` _returnvalue 0)
  (bind _returnvalue_2 (`|CreateWidget` "/Game/Bleuprints/BP_ObjectHPWidgetHUD.BP_ObjectHPWidgetHUD_C"))
  (`UserWidget.AddToViewport` _returnvalue_2 0)
  (set `self.ObjectHPWidget` _returnvalue_2)
  (set `self.GamePanelWidget` _returnvalue)
  (set `/Game/Bleuprints/BP_ObjectHPWidgetHUD.Bottom Panel Shop` (`/Game/Bleuprints/BP_GamePanelWidgetHUD.Bottom_panel_shop` _returnvalue) _returnvalue_2)
  (bind _returnvalue_3 (`|CreateWidget` "/Game/Bleuprints/BP_ObjectHPWidgetHUD.BP_ObjectHPWidgetHUD_C"))
  (`UserWidget.AddToViewport` _returnvalue_3 0))

(event `/Game/Bleuprints/BP_SelectingInterface.Start Selection`
  (bind (_locationx _locationy) (`WidgetLayoutLibrary.GetMousePositionScaledByDPI` (`GameplayStatics.GetPlayerController` 0)))
  ;[1 1 1] drag selection
  (set `self.PointA` (`KismetMathLibrary.MakeVector2D` _locationx _locationy))
  (set `self.isDrawing` true))

(event `/Game/Bleuprints/BP_SelectingInterface.Stop Selection`
  ;[1 1 1] drag selection
  (set `self.isDrawing` false)
  (`PlayerCameraControllerPawn.UnselectUnits` (`self.BP_PlayerControllerPawn`))
  (for _array_element (`self.SelectionOfUnits`)
    (bind _asunit_spawn (cast `UnitSpawn` _array_element)
      (:`then`
        (`KismetArrayLibrary.Array_AddUnique` (`PlayerCameraControllerPawn.Units` (`self.BP_PlayerControllerPawn`)) _asunit_spawn)
        (`UnitSpawn.CylinderHideShow` _asunit_spawn))
      (:`CastFailed`
        (`KismetSystemLibrary.PrintString` "Failed to cast - BP_GamePanelHUD" true true (struct :`G` 0.66 :`B` 1.0 :`A` 1.0) 55.0)))))

(event `self.ReceiveDrawHUD`
  (params (SizeX :type Integer) (SizeY :type Integer))
  (bind (_pointa_x _pointa_y) (`KismetMathLibrary.BreakVector2D` (`self.PointA`)))
  (bind (_pointb_x _pointb_y) (`KismetMathLibrary.BreakVector2D` (`self.PointB`)))
  (bind (_locationx _locationy) (`WidgetLayoutLibrary.GetMousePositionScaledByDPI` (`GameplayStatics.GetPlayerController` 0)))
  ;[1 1 1] drag selection
  (if (`self.isDrawing`)
    (set `self.PointB` (`KismetMathLibrary.MakeVector2D` _locationx _locationy))
    (`self.DrawRect` (struct :`R` 0.983333 :`G` 0.134561 :`A` 0.5) _pointa_x _pointa_y (- _pointb_x _pointa_x) (- _pointb_y _pointa_y))
    (set `self.SelectionOfUnits` (`self.GetActorsInSelectionRectangle` "/Script/COLONISE3d.UnitSpawn" (`self.PointA`) (`self.PointB`) false))))

(fn `Get_BP_PlayerControllerPawn`
  (params (BP_PlayerControllerPawn :type "/Game/Bleuprints/BP_PlayerCameraControllerPawn Object Reference"))
  (set `self.BP_PlayerControllerPawn` BP_PlayerControllerPawn))

(fn `UserConstructionScript`)