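; BP_MainWarehouseSpawn is a main warehouse that holds the Wood, Stone and Food stockpiles, seeded with starting amounts on BeginPlay.
; When a BP_UnitSpawn enters its box trigger, the warehouse adds the unit's carried resources to its totals and zeroes the unit's amounts.
; Clicking the warehouse shows the HUD's bottom shop panel and sets a flag; the logic to hide it again is disconnected.
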(event `self.ReceiveBeginPlay`
  (set `self.Wood` 500.0)
  (set `self.Stone` 400.0)
  (set `self.Food` 500.0))

(event `self.Box.OnComponentBeginOverlap`
  (params (OverlappedComponent :type "PrimitiveComponent Object Reference") (OtherActor :type "Actor Object Reference") (OtherComp :type "PrimitiveComponent Object Reference") (OtherBodyIndex :type Integer) (bFromSweep :type Boolean) (SweepResult :type "HitResult Structure (by ref)"))
  (bind _unit (`self.Unit`))
  (if (== (`GameplayStatics.GetObjectClass` OtherActor) "/Game/Bleuprints/BP_UnitSpawn.BP_UnitSpawn_C")
    (bind _asbp_unit_spawn (cast `/Game/Bleuprints/BP_UnitSpawn` OtherActor))
    (set `self.Unit` _asbp_unit_spawn)
    ;[1 1 1] add unit mats to my mats
    (set `self.Wood` (+ (`self.Wood`) (`UnitSpawn.Wood` _unit)))
    (set `self.Food` (+ (`self.Food`) (`UnitSpawn.Food` _unit)))
    (set `self.Stone` (+ (`self.Stone`) (`UnitSpawn.Stone` _unit)))
    ;[1 1 1] reset given resources
    (set `UnitSpawn.Wood` 0.0 _unit)
    (set `UnitSpawn.Food` 0.0 _unit)
    (set `UnitSpawn.Stone` 0.0 _unit)))

(event `self.MainWarehouse.OnClicked`
  (params (TouchedComponent :type "PrimitiveComponent Object Reference") (ButtonPressed :type "Key Structure"))
  (bind _gamepanelwidgethud (`self.GamePanelWidgetHUD`))
  ;[1 1 1] Show/Hide bottom panel (shop)
  (if (not (`self.Bottom_panel_shop`))
    (bind _output_get (set `self.GamePanelWidgetHUD` _gamepanelwidgethud))
    (bind _output_get_2 (set `/Game/Bleuprints/BP_GamePanelWidgetHUD.Bottom_panel_shop` (`/Game/Bleuprints/BP_GamePanelWidgetHUD.Bottom_panel_shop` _gamepanelwidgethud) _output_get))
    (`Widget.SetVisibility` _output_get_2 "Visible")
    (set `self.Bottom_panel_shop` true)))

(fn `UserConstructionScript`)