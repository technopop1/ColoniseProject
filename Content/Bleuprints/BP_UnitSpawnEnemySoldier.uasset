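; Enemy soldier unit for an RTS-style game that cannot gather and automatically chases and attacks nearby player units.
; Sphere overlaps keep an array of worker, soldier and range soldier units within reach.
; A looping timer targets the nearest one, subtracts its Health directly and destroys it when low, with no separate attack-range check.
; While targets exist, Tick drives AI MoveToLocation toward the target's last sampled position.
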(event `self.ReceiveBeginPlay`
  ;[1 1 1] make soldier unable to gather
  (set `self.GatheringSpeed` 0.0)
  (set `self.Health` 300.0)
  (set `self.AttackDmg` 25.0)
  (`KismetSystemLibrary.K2_SetTimerDelegate` (delegate `Attack closest units`) 1.5 true))

(event `Attack closest units`
  (bind _unitarray (`self.UnitArray`))
  (bind (_distance _returnvalue) (`GameplayStatics.FindNearestActor` (`self.K2_GetActorLocation` self) _unitarray))
  ;[1 1 1] Attack closest unit
  (if (> (`KismetArrayLibrary.Array_Length` _unitarray) 0)
    (set `self.FollowUnitToAttack` true)
    (if (`KismetSystemLibrary.IsValid` _returnvalue)
      (bind _asunit_spawn (cast `UnitSpawn` _returnvalue))
      (set `self.Destination` (`self.K2_GetActorLocation` _asunit_spawn))
      (bind _returnvalue_2 (- (`UnitSpawn.Health` _asunit_spawn) (`self.AttackDmg`)))
      (set `UnitSpawn.Health` _returnvalue_2 _asunit_spawn)
      (if (<= _returnvalue_2 0.0)
        (`self.K2_DestroyActor` _asunit_spawn)))
    (else
      (set `self.FollowUnitToAttack` false))))

(event `self.ReceiveTick`
  (params (DeltaSeconds :type "Float (single-precision)"))
  (if (`self.FollowUnitToAttack`)
    (`self.MoveToDestination`)))

(event `self.Sphere.OnComponentBeginOverlap`
  (params (OverlappedComponent :type "PrimitiveComponent Object Reference") (OtherActor :type "Actor Object Reference") (OtherComp :type "PrimitiveComponent Object Reference") (OtherBodyIndex :type Integer) (bFromSweep :type Boolean) (SweepResult :type "HitResult Structure (by ref)"))
  (bind _unitarray (`self.UnitArray`))
  ;[1 1 1] Add Units closed to me to arrays
  (if (== (`GameplayStatics.GetObjectClass` OtherActor) "/Game/Bleuprints/BP_UnitSpawn.BP_UnitSpawn_C")
    (bind _asunit_spawn (cast `UnitSpawn` OtherActor))
    (`KismetArrayLibrary.Array_Add` _unitarray _asunit_spawn)
    (elif (== (`GameplayStatics.GetObjectClass` OtherActor) "/Game/Bleuprints/BP_UnitSpawnSoldier.BP_UnitSpawnSoldier_C")
      (bind _asunit_spawn_2 (cast `UnitSpawn` OtherActor))
      (`KismetArrayLibrary.Array_Add` _unitarray _asunit_spawn_2)
      (elif (== (`GameplayStatics.GetObjectClass` OtherActor) "/Game/Bleuprints/BP_UnitSpawnRangeSoldier.BP_UnitSpawnRangeSoldier_C")
        (bind _asunit_spawn_3 (cast `UnitSpawn` OtherActor))
        (`KismetArrayLibrary.Array_Add` _unitarray _asunit_spawn_3)))))

(event `self.Sphere.OnComponentEndOverlap`
  (params (OverlappedComponent :type "PrimitiveComponent Object Reference") (OtherActor :type "Actor Object Reference") (OtherComp :type "PrimitiveComponent Object Reference") (OtherBodyIndex :type Integer))
  (bind _unitarray (`self.UnitArray`))
  ;[1 1 1] Add Units closed to me to arrays
  (if (== (`GameplayStatics.GetObjectClass` OtherActor) "/Game/Bleuprints/BP_UnitSpawn.BP_UnitSpawn_C")
    (bind _asunit_spawn (cast `UnitSpawn` OtherActor))
    (`KismetArrayLibrary.Array_RemoveItem` _unitarray _asunit_spawn)
    (elif (== (`GameplayStatics.GetObjectClass` OtherActor) "/Game/Bleuprints/BP_UnitSpawnSoldier.BP_UnitSpawnSoldier_C")
      (bind _asunit_spawn_2 (cast `UnitSpawn` OtherActor))
      (`KismetArrayLibrary.Array_RemoveItem` _unitarray _asunit_spawn_2)
      (elif (== (`GameplayStatics.GetObjectClass` OtherActor) "/Game/Bleuprints/BP_UnitSpawnRangeSoldier.BP_UnitSpawnRangeSoldier_C")
        (bind _asunit_spawn_3 (cast `UnitSpawn` OtherActor))
        (`KismetArrayLibrary.Array_RemoveItem` _unitarray _asunit_spawn_3)))))

(fn `AcceptableRadiusOfMove`
  (set `self.RadiusStopMove` 1.0)
  (return))

(fn `MoveToDestination`
  (bind _destination (`self.Destination`))
  (bind _radiusstopmove (`self.RadiusStopMove`))
  (bind _returnvalue (`AIBlueprintHelperLibrary.GetAIController` self))
  (if (== _destination (`KismetMathLibrary.Vector_Zero`) :`ErrorTolerance` 1.0)
    _
    (elif (`KismetSystemLibrary.IsValid` _returnvalue)
      (set `CharacterMovementComponent.MaxWalkSpeed` 300.0 (`self.CharacterMovement`))
      (`self.AcceptableRadiusOfMove`)
      (`AIController.MoveToLocation` _returnvalue _destination _radiusstopmove true true false true null true)
      (if (== _destination (`self.K2_GetActorLocation` self) :`ErrorTolerance` _radiusstopmove)
        (`SkeletalMeshComponent.SetAnimation` (`self.Mesh`) "/Game/Mannequin/Animations/ThirdPersonIdle.ThirdPersonIdle")
        (if (`self.bIfWarehouse`)
          (if (`KismetSystemLibrary.IsValid` (`self.ClickedTree`))
            (set `self.bUnitMove` true :!label _label)
            (elif (`KismetSystemLibrary.IsValid` (`self.ClickedRock`))
              (goto _label)
              (else
                _)))
          (else
            (set `self.bUnitMove` false)))
        (return)
        (else
          (return)))
      (else
        _)))
  (return))

(fn `UserConstructionScript`)